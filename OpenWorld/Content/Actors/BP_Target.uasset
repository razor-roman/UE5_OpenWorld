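; BP_Target is a knock-down target actor that tips over when hit and then stands back up.
; A BP_Projectile hit on the mesh while IsReady, or an OnHit event that skips that check, clears IsReady and plays the Down timeline to pitch the mesh.
; A one-second Delay on that timeline's Update pin then triggers a second timeline in reverse to raise it and sets IsReady again.
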(event OnComponentHit(StaticMesh)
  (params (HitComponent :type Primitive%20Component%20Object%20Reference) (OtherActor :type Actor%20Object%20Reference) (OtherComp :type Primitive%20Component%20Object%20Reference) (NormalImpulse :type Vector :default "0, 0, 0") (Hit :type Hit%20Result%20Structure%20%28by%20ref%29))
  (if (and (== (Utilities|GetClass OtherActor) "/Game/Actors/BP_Projectile.BP_Projectile_C") (Variables|Default|GetIsReady))
    (CallFunction|TargetDown)
    (Variables|Default|SetIsReady false)))

(event Custom|OnHit
  (CallFunction|TargetDown)
  (Variables|Default|SetIsReady false))

(event Custom|TargetDown
  (bind _newtrack_0 (Timeline|Down PlayFromStart)
    (:Update
      (Transformation|SetRelativeRotation (Variables|Components|GetStaticMesh) (Math|Rotator|MakeRotator 0.0 (* _newtrack_0 9e+01) 0.0) false false)
      (Utilities|FlowControl|Delay 1.0)
      (CallFunction|TargetUp)
      (Variables|Default|SetIsReady true))))

(event Custom|TargetUp
  (bind _newtrack_0 (Timeline|Timeline_0 ReverseFromEnd)
    (:Update
      (Transformation|SetRelativeRotation (Variables|Components|GetStaticMesh) (Math|Rotator|MakeRotator 0.0 (* _newtrack_0 9e+01) 0.0) false false))))

(event EventBeginPlay)

(event Collision|EventActorBeginOverlap
  (params (OtherActor :type Actor%20Object%20Reference)))

(event EventTick
  (params (DeltaSeconds :type Float%20%28single-precision%29)))

(fn ConstructionScript)
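; BP_Grenade is a timed grenade actor that explodes one second after BeginPlay.
; Explode runs a multi sphere trace on Visibility with persistent debug drawing, from the actor's location to that location multiplied by a local variable.
; For each StaticMeshActor hit, it prints the hit location and fires the RadialForce impulse, so the impulse can fire several times per explosion.
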(event EventBeginPlay
  (Utilities|FlowControl|Delay 1.0)
  (Utilities|FlowControl|DoOnce false
    (:Completed
      (CallFunction|Explode))))

(event Collision|EventActorBeginOverlap
  (params (OtherActor :type Actor%20Object%20Reference)))

(event EventTick
  (params (DeltaSeconds :type Float%20%28single-precision%29)))

(fn ConstructionScript)

(fn Explode
  (bind _returnvalue (Transformation|GetActorLocation))
  (bind (_outhits _returnvalue_2) (Collision|MultiSphereTraceByChannel _returnvalue (* _returnvalue (LocalVariables|GetNewLocalVar_0)) (Variables|Default|GetRadius) "TraceTypeQuery1" false 0 "Persistent"))
  (if _returnvalue_2
    (for _array_element _outhits
      (Utilities|Casting|CastToStaticMeshActor (.HitActor (Collision|BreakHitResult _array_element)))
      (Development|PrintString (Utilities|String|ToString(Vector) (.Location (Collision|BreakHitResult _array_element))))
      (Class|RadialForceComponent|FireImpulse (Variables|Default|GetRadialForce)))))
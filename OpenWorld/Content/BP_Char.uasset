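; Player character with camera-yaw-relative movement and key-driven test actions for grenades, item tracing and physics animation.
; Q and Resume share a FlipFlop that toggles the WBP_Main menu, cursor and input mode, with the game left unpaused.
; F spawns and launches BP_Grenade, while E box-traces and prints the hit actor's name.
; R ragdolls the mesh, and T applies a physical animation profile to bodies below a chosen bone.
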(event Custom|Resume
  (bind _returnvalue (Game|GetPlayerController 0))
  (bind _returnvalue_2 (Game|GetPlayerController 0))
  ;[1 1 1] Open/Close Menu
  (Utilities|FlowControl|FlipFlop
    (:A
      (Game|SetGamePaused false)
      (bind _returnvalue_3 (UserInterface|CreateWidget "/Game/UI/WBP_Main.WBP_Main_C"))
      (bind _output_get (Variables|Default|SetPauseWidget _returnvalue_3))
      (UserInterface|Viewport|AddtoPlayerScreen _output_get)
      (Variables|/Script/Engine.PlayerController|SetbShowMouseCursor _returnvalue true)
      (Input|SetInputModeGameandUI _returnvalue (Variables|Default|GetPauseWidget) "DoNotLock" true))
    (:B
      (Game|SetGamePaused false)
      (Widget|RemovefromParent (Variables|Default|GetPauseWidget))
      (Variables|/Script/Engine.PlayerController|SetbShowMouseCursor _returnvalue_2 false)
      (Input|SetInputModeGameOnly _returnvalue_2))))

(event EventBeginPlay
  (Class|PhysicalAnimationComponent|SetStrengthMultiplyer (Variables|Default|GetPhysicalAnimation) 0.0))

(event Collision|EventActorBeginOverlap
  (params (OtherActor :type Actor%20Object%20Reference)))

(event EventTick
  (params (DeltaSeconds :type Float%20%28single-precision%29)))

(event Input|AxisEvents|InputAxisLookUp
  (params (AxisValue :type Float%20%28single-precision%29))
  ;[1 1 1] Controller
  (Pawn|Input|AddControllerPitchInput AxisValue))

(event Input|AxisEvents|InputAxisTurn
  (params (AxisValue :type Float%20%28single-precision%29))
  ;[1 1 1] Controller
  (Pawn|Input|AddControllerYawInput AxisValue))

(event Input|AxisEvents|InputAxisForward
  (params (AxisValue :type Float%20%28single-precision%29))
  ;[1 1 1] Controller
  (Pawn|Input|AddMovementInput (Math|Vector|GetForwardVector (Math|Rotator|MakeRotator 0.0 0.0 (.Yaw (Math|Rotator|BreakRotator (Pawn|GetControlRotation :!class /Script/Engine.Pawn))))) AxisValue false))

(event Input|AxisEvents|InputAxisRight
  (params (AxisValue :type Float%20%28single-precision%29))
  ;[1 1 1] Controller
  (Pawn|Input|AddMovementInput (Math|Vector|GetRightVector (Math|Rotator|MakeRotator 0.0 0.0 (.Yaw (Math|Rotator|BreakRotator (Pawn|GetControlRotation :!class /Script/Engine.Pawn))))) AxisValue false))

(event Input|KeyboardEvents|Q
  (params (Key :type Key%20Structure :default "None"))
  (bind _returnvalue (Game|GetPlayerController 0))
  (bind _returnvalue_2 (Game|GetPlayerController 0))
  ;[1 1 1] Open/Close Menu
  (:Pressed
    (Utilities|FlowControl|FlipFlop
      (:A
        (Game|SetGamePaused false)
        (bind _returnvalue_3 (UserInterface|CreateWidget "/Game/UI/WBP_Main.WBP_Main_C"))
        (bind _output_get (Variables|Default|SetPauseWidget _returnvalue_3))
        (UserInterface|Viewport|AddtoPlayerScreen _output_get)
        (Variables|/Script/Engine.PlayerController|SetbShowMouseCursor _returnvalue true)
        (Input|SetInputModeGameandUI _returnvalue (Variables|Default|GetPauseWidget) "DoNotLock" true))
      (:B
        (Game|SetGamePaused false)
        (Widget|RemovefromParent (Variables|Default|GetPauseWidget))
        (Variables|/Script/Engine.PlayerController|SetbShowMouseCursor _returnvalue_2 false)
        (Input|SetInputModeGameOnly _returnvalue_2)))))

(event Input|KeyboardEvents|F
  (params (Key :type Key%20Structure :default "None"))
  (bind _returnvalue (Transformation|GetActorTransform))
  ;[1 1 1] Spawn Grenade
  (:Pressed
    (bind _returnvalue_2 (Game|SpawnActorfromClass "/Game/Actors/BP_Grenade.BP_Grenade_C" (Math|Transform|MakeTransform (+ (.location _returnvalue) (* (Math|Vector|GetForwardVector (Variables|Character|GetMesh)) (Variables|Default|GetAddToForward))) (.rotation _returnvalue) (Variables|Default|GetSpawn%20Transform%20Scale)) "AdjustIfPossibleButAlwaysSpawn" 0 0))
    (bind _output_get (Variables|Default|SetGrenade _returnvalue_2))
    (Physics|AddImpulse (Variables|/Game/Actors/BP_Grenade.BP_Grenade_C|GetSphere _output_get) (* (Transformation|GetActorForwardVector) (Variables|Default|GetImpulseMulti)) "None" false)))

(event Input|KeyboardEvents|E
  (params (Key :type Key%20Structure :default "None"))
  (bind _capsulecomponent (Variables|Collision|GetCapsuleComponent))
  ;[1 1 1] Trace for items
  (:Pressed
    (bind (_outhit _returnvalue) (Collision|BoxTraceByChannel (Transformation|GetWorldLocation _capsulecomponent) (* (Math|Vector|GetForwardVector _capsulecomponent) (Variables|Default|GetAddToForward)) "0, 0, 0" "0, 0, 0" "TraceTypeQuery2" false 0 "Persistent"))
    (if _returnvalue
      (Development|PrintString (Utilities|GetDisplayName (.HitActor (Collision|BreakHitResult _outhit)))))))

(event Input|KeyboardEvents|R
  (params (Key :type Key%20Structure :default "None"))
  ;[1 1 1] RagDoll
  (:Pressed
    (Physics|SetSimulatePhysics (Variables|Character|GetMesh) true)
    (Pawn|Components|CharacterMovement|DisableMovement (Variables|Character|GetCharacterMovement))))

(event Input|KeyboardEvents|T
  (params (Key :type Key%20Structure :default "None"))
  (bind _physicalanimation (Variables|Default|GetPhysicalAnimation))
  (bind _bodyname (Variables|Default|GetBodyName))
  (:Pressed
    (Class|PhysicalAnimationComponent|SetSkeletalMeshComponent _physicalanimation (Variables|Character|GetMesh))
    (Class|PhysicalAnimationComponent|ApplyPhysicalAnimationProfileBelow _physicalanimation _bodyname "AnimProfile" false false)
    (Class|SkeletalMeshComponent|SetAllBodiesBelowSimulatePhysics (Variables|Character|GetMesh) _bodyname true false)
    (Class|PhysicalAnimationComponent|SetStrengthMultiplyer (Variables|Default|GetPhysicalAnimation) 5e+01)))

(fn ConstructionScript)
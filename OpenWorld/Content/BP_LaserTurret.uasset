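; Player-controlled laser turret that yaws with the Right input axis and fires at dummy AI and targets on left click.
; Firing plays a gun animation, waits a fixed delay, then spawns a Niagara laser and line-traces forward from ShootingPoint with persistent debug drawing.
; Hits call PhysicsOn on BP_DummyAI or OnHit on BP_Target, each incrementing and printing the score.
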(event EventBeginPlay)

(event Collision|EventActorBeginOverlap
  (params (OtherActor :type Actor%20Object%20Reference)))

(event EventTick
  (params (DeltaSeconds :type Float%20%28single-precision%29)))

(event Input|AxisEvents|InputAxisRight
  (params (AxisValue :type Float%20%28single-precision%29))
  (bind _output_get (Variables|Default|SetCurrentHRotation (+ (* AxisValue (Utilities|Time|GetWorldDeltaSeconds) (Variables|Default|GetHRotationSpeed)) (Variables|Default|GetCurrentHRotation))))
  (Transformation|SetActorRotation (Math|Rotator|MakeRotator 0.0 0.0 _output_get)))

(event Input|MouseEvents|LeftMouseButton
  (params (Key :type Key%20Structure :default "None"))
  (bind _shootingpoint (Variables|Default|GetShootingPoint))
  (bind _shootingpoint_2 (Variables|Default|GetShootingPoint))
  (bind _returnvalue (Transformation|GetWorldLocation _shootingpoint))
  (:Pressed
    (Components|Animation|PlayAnimation (Variables|Default|GetSkeletalMesh) "/Game/CSC/Animations/Anim_CSC_Gun4.Anim_CSC_Gun4" false)
    (Utilities|FlowControl|Delay 1.95)
    (bind _returnvalue_2 (Niagara|SpawnSystematLocation "/Game/FX/FX_LaserShot.FX_LaserShot" (Transformation|GetWorldLocation _shootingpoint_2) (Transformation|GetWorldRotation _shootingpoint_2) "1.000000,1.000000,1.000000" true true "AutoRelease"))
    (Variables|Default|SetLaserEffect _returnvalue_2)
    (bind (_outhit _returnvalue_3) (Collision|LineTraceByChannel _returnvalue (+ _returnvalue (* (Math|Vector|GetForwardVector _shootingpoint) (Variables|Default|GetShotRange))) "TraceTypeQuery1" false 0 "Persistent"))
    (if _returnvalue_3
      (Utilities|FlowControl|Sequence
        (:then_0
          (bind _asbp_dummy_ai (Utilities|Casting|CastToBP_DummyAI (.HitActor (Collision|BreakHitResult _outhit))))
          (Default|Physicson _asbp_dummy_ai))
        (:then_1
          (bind _asbp_target (Utilities|Casting|CastToBP_Target (.HitActor (Collision|BreakHitResult _outhit))))
          (Default|OnHit _asbp_target)))
      (bind _output_get (Variables|Default|SetScore (+ (Variables|Default|GetScore) 1)))
      (Development|PrintString (Utilities|String|ToString(Byte) _output_get)))))

(fn ConstructionScript)
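; Player-controlled turret that aims with input axes and fires projectiles on left mouse click.
; On BeginPlay it caches the skeletal mesh's ABP_Turel anim instance.
; Axis input accumulates frame-rate-independent yaw and clamped pitch values and pushes them to the AnimBP, which presumably poses the turret.
; Left click spawns BP_Projectile at the ProjectileSpawnLocation component's world transform.
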(event EventBeginPlay
  (bind _asabp_turel (Utilities|Casting|CastToABP_Turel (Components|SkeletalMesh|GetAnimInstance (Variables|Default|GetSKTurel))))
  (Variables|Default|SetABPInstance _asabp_turel))

(event Collision|EventActorBeginOverlap
  (params (OtherActor :type Actor%20Object%20Reference)))

(event EventTick
  (params (DeltaSeconds :type Float%20%28single-precision%29)))

(event Input|AxisEvents|InputAxisRight
  (params (AxisValue :type Float%20%28single-precision%29))
  (bind _output_get (Variables|Default|SetCurrentHRotation (+ (* AxisValue (Utilities|Time|GetWorldDeltaSeconds) (Variables|Default|GetHRotationSpeed)) (Variables|Default|GetCurrentHRotation))))
  (Variables|/Game/SkeletalMesh/ABP_Turel.ABP_Turel_C|SetHrotation (Variables|Default|GetABPInstance) _output_get))

(event Input|AxisEvents|InputAxisForward
  (params (AxisValue :type Float%20%28single-precision%29))
  (bind _output_get (Variables|Default|SetCurrentVRotation (Math|Float|Clamp(Float) (+ (* AxisValue (Utilities|Time|GetWorldDeltaSeconds) (Variables|Default|GetVRotationSpeed)) (Variables|Default|GetCurrentVRotation)) -4e+01 1e+01)))
  (Variables|/Game/SkeletalMesh/ABP_Turel.ABP_Turel_C|SetVRotation (Variables|Default|GetABPInstance) _output_get))

(event Input|MouseEvents|LeftMouseButton
  (params (Key :type Key%20Structure :default "None"))
  (bind _projectilespawnlocation (Variables|Default|GetProjectileSpawnLocation))
  (bind _returnvalue (Transformation|GetWorldTransform _projectilespawnlocation))
  (:Pressed
    (Game|SpawnActorfromClass "/Game/Actors/BP_Projectile.BP_Projectile_C" (Math|Transform|MakeTransform (.location _returnvalue) (.rotation _returnvalue) "1.000000,1.000000,1.000000") "Undefined" 0 0)))

(fn ConstructionScript)